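; BP_AudioManager is an audio manager actor that starts the background music for the current level.
; On BeginPlay it switches on the current level name, choosing MainMenuMusic for Main Menu and GameMusic for Lvl Timetrial.
; The chosen sound is assigned to AudioComp, played from the start, then scaled by the Volume variable.
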(event EventBeginPlay
  (bind _returnvalue (Game|GetCurrentLevelName true))
  (switch string _returnvalue
    (:MainMenu
      (Audio|Components|Audio|SetSound (Variables|Default|GetAudioComp) (Variables|Default|GetMainMenuMusic))
      (Audio|Components|Audio|Play (Variables|Default|GetAudioComp) 0.0)
      (Audio|Components|Audio|SetVolumeMultiplier (Variables|Default|GetAudioComp) (Variables|Default|GetVolume) :!class /Script/Engine.AudioComponent))
    (:Lvl_Timetrial
      (Audio|Components|Audio|SetSound (Variables|Default|GetAudioComp) (Variables|Default|GetGameMusic))
      (Audio|Components|Audio|Play (Variables|Default|GetAudioComp) 0.0)
      (Audio|Components|Audio|SetVolumeMultiplier (Variables|Default|GetAudioComp) (Variables|Default|GetVolume) :!class /Script/Engine.AudioComponent))))

(event Collision|EventActorBeginOverlap
  (params (OtherActor :type Actor%20Object%20Reference)))

(event EventTick
  (params (DeltaSeconds :type Float%20%28single-precision%29)))

(fn ConstructionScript)