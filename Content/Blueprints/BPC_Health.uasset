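; Health component that tracks its owning actor's current health and death state.
; On BeginPlay it resets health to maximum and binds to the owner's OnTakeAnyDamage event.
; Incoming damage is subtracted with clamping and broadcast through OnHealthChanged, with debug prints of damage and remaining health.
; At zero health it sets a dead flag that blocks further damage, prints the death and calls OnDeath.
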(event Custom|HandleDamageEvent
  (params (DamagedActor :type Actor%20Object%20Reference) (Damage :type Float%20%28single-precision%29) (DamageType :type Damage%20Type%20Object%20Reference) (InstigatedBy :type Controller%20Object%20Reference) (DamageCauser :type Actor%20Object%20Reference))
  (CallFunction|CustomHandleDamage Damage))

(event EventBeginPlay
  (Variables|Health|SetCurrentHealth (Variables|Health|GetMaxHealth))
  (Variables|Health|SetIsDead false)
  (EventDispatchers|BindEventtoOnTakeAnyDamage (Components|GetOwner) (delegate Custom|HandleDamageEvent)))

(fn CustomHandleDamage
  (params (Damage :type Float%20%28double-precision%29))
  (if (Variables|Health|GetIsDead)
    (return)
    (else
      (bind _output_get (Variables|Health|SetCurrentHealth (Math|Float|Clamp(Float) (- (Variables|Health|GetCurrentHealth) Damage) 0.0 (Variables|Health|GetMaxHealth))))
      (Default|CallOnHealthChanged)
      (Development|PrintString (Utilities|String|Append "Dealt damage: " (Utilities|String|ToString(Float) Damage) ", New HP: " (Utilities|String|ToString(Float) _output_get)))
      (if (<= _output_get 0.0)
        (Variables|Health|SetIsDead true)
        (Development|PrintString (Utilities|String|Append (Utilities|GetDisplayName (Components|GetOwner)) " is dead"))
        (Default|CallOnDeath)))))