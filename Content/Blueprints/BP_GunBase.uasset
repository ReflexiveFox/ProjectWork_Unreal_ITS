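; Base gun Blueprint with automatic fire and an overheat mechanic; DoFire only prints a debug message.
; StartFire fires immediately and starts a looping fire timer, with each shot adding heat through TryFire.
; Reaching max heat stops firing and blocks shooting until heat cools back to zero.
; StopFire starts a looping cooldown timer, with CoolRate serving as both its interval and heat decrement.
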(event Custom|OnWeaponTimerFinished
  (GenericWeapon|TryFire))

(event Custom|OnCooldownRateFinished
  (GenericWeapon|DecreaseHeat))

(event EventBeginPlay
  (GenericWeapon|InitializeWeapon))

(fn ConstructionScript)

(fn StartFire
  (if (GenericWeapon|CanWeaponShoot)
    (Variables|GenericWeapon|SetIsFiring true)
    (GenericWeapon|TryFire)
    (bind _returnvalue (Utilities|Time|SetTimerbyEvent (EventDispatchers|CreateEvent :!event Custom|OnWeaponTimerFinished) (Variables|GenericWeapon|GetFireRate) true))
    (Variables|GenericWeapon|SetFireTimerHandle _returnvalue)
    (Utilities|Time|ClearandInvalidateTimerbyHandle (Variables|GenericWeapon|GetCooldownTimerHandle))
    (else
      (return))))

(fn StopFire
  (Variables|GenericWeapon|SetIsFiring false)
  (Utilities|Time|ClearandInvalidateTimerbyHandle (Variables|GenericWeapon|GetFireTimerHandle))
  (bind _returnvalue (Utilities|Time|SetTimerbyEvent (EventDispatchers|CreateEvent :!event Custom|OnCooldownRateFinished) (Variables|GenericWeapon|GetCoolRate) true))
  (Variables|GenericWeapon|SetCooldownTimerHandle _returnvalue))

(fn TryFire
  (if (GenericWeapon|CanWeaponShoot)
    (Development|PrintString "I am firing")
    (GenericWeapon|DoFire)
    (GenericWeapon|IncreaseHeat)
    (else
      (return))))

(fn DoFire
  (Development|PrintString "DoFire in GunBase"))

(fn IncreaseHeat
  (bind _maxheat (Variables|GenericWeapon|GetMaxHeat))
  (bind _output_get (Variables|GenericWeapon|SetCurrentHeat (Math|Float|Clamp(Float) (+ (Variables|GenericWeapon|GetCurrentHeat) (Variables|GenericWeapon|GetHeatPerShot)) 0.0 _maxheat)))
  (if (>= _output_get _maxheat)
    (Utilities|FlowControl|Sequence
      (:then_0
        (Variables|GenericWeapon|SetIsOverheated true))
      (:then_1
        (Variables|GenericWeapon|SetCanShoot false))
      (:then_2
        (GenericWeapon|StopFire)))))

(fn InitializeWeapon
  (Variables|GenericWeapon|SetCanShoot true)
  (Variables|GenericWeapon|SetIsFiring false)
  (Variables|GenericWeapon|SetIsOverheated false))

(fn DecreaseHeat
  (bind _output_get (Variables|GenericWeapon|SetCurrentHeat (Math|Float|Clamp(Float) (- (Variables|GenericWeapon|GetCurrentHeat) (Variables|GenericWeapon|GetCoolRate)) 0.0 (Variables|GenericWeapon|GetMaxHeat))))
  (if (<= _output_get 0.0)
    (Utilities|FlowControl|Sequence
      (:then_0
        (Variables|GenericWeapon|SetIsOverheated false))
      (:then_1
        (Variables|GenericWeapon|SetCanShoot true))
      (:then_2
        (if (Variables|GenericWeapon|GetIsFiring)
          (GenericWeapon|TryFire))))))

(fn CanWeaponShoot
  (return (and (not (Variables|GenericWeapon|GetIsOverheated)) (Variables|GenericWeapon|GetCanShoot))))

(fn GetHeatPercent
  (return (Math|Float|Clamp(Float) (/ (Variables|GenericWeapon|GetCurrentHeat) (Variables|GenericWeapon|GetMaxHeat)))))

(fn GetFireRate
  (return (Variables|GenericWeapon|GetFireRate)))