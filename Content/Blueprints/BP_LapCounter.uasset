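; BP_LapCounter is a trigger actor that counts laps for the sports car vehicle and signals when the race laps are done.
; The first overlap only sets IsFirstTime, whose name reads inverted, and later overlaps increment MyLaps through a DoOnce.
; It calls OnLapsUpdated, then resets the DoOnce after a delay to block repeat counts.
; Exceeding MaxLaps calls OnLapsFinished and leaves the DoOnce closed.
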(event OnComponentBeginOverlap(Trigger)
  (params (OverlappedComponent :type Primitive%20Component%20Object%20Reference) (OtherActor :type Actor%20Object%20Reference) (OtherComp :type Primitive%20Component%20Object%20Reference) (OtherBodyIndex :type Integer) (bFromSweep :type Boolean) (SweepResult :type Hit%20Result%20Structure%20%28by%20ref%29))
  (bind _mylaps (Variables|Default|GetMyLaps))
  (bind _maxlaps (Variables|Default|GetMaxLaps))
  (Utilities|Casting|CastToBP_VehicleAdvSportsCar OtherActor)
  (if (Variables|Default|GetIsFirstTime)
    (Development|PrintString "Its not first time passing, count lap")
    (Utilities|FlowControl|DoOnce false :!label _label
      (:Completed
        (bind _result (Math|Integer|IncrementInt _mylaps)
          (:%20%20
            (if (> _result _maxlaps)
              ;[0.15 0.15 0.15 0.5] Update Game Mode
              (Default|CallOnLapsFinished)
              (else
                (Default|CallOnLapsUpdated _mylaps _maxlaps)
                (Utilities|FlowControl|Delay 2e+01)
                (goto _label Reset)))))))
    (else
      (Development|PrintString "Its first time passing, dont count")
      (Variables|Default|SetIsFirstTime true))))

(event EventBeginPlay)

(event Collision|EventActorBeginOverlap
  (params (OtherActor :type Actor%20Object%20Reference)))

(event EventTick
  (params (DeltaSeconds :type Float%20%28single-precision%29)))

(fn ConstructionScript)