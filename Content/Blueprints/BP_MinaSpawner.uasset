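; Spawner actor that places BP_Mina mines, extending a parent class's firing logic and starting fire on BeginPlay.
; Each DoFire calls SpawnMina, which runs a debug-drawn Visibility line trace with an unset start and an end one unit down from world origin.
; On a hit, it spawns a mine at the impact with its X axis along the surface normal; otherwise it only prints a failure message.
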(event EventBeginPlay
  (CallFunction|StartFire))

(fn ConstructionScript
  (|CallParentFunction))

(fn DoFire
  (|CallParentFunction)
  (GenericWeapon|SpawnMina))

(fn SpawnMina
  (Development|PrintString "Spawna la mina!")
  (bind _outhit (Collision|LineTraceByChannel "0, 0, 0" (* (Math|Vector|VectorUp) (Math|Conversions|ToVector(Float) -1.0)) "TraceTypeQuery1" false 0 "ForDuration"))
  (if (.bblockinghit _outhit)
    (Development|PrintString "Spawning mina...")
    (Game|SpawnActorfromClass "/Game/Blueprints/BP_Mina.BP_Mina_C" (Math|Transform|MakeTransform (.location _outhit) (Math|Conversions|RotationFromXVector (.normal _outhit))) "AdjustIfPossibleButAlwaysSpawn" "MultiplyWithRoot" 0 0.1 0)
    (else
      (Development|PrintString "Did not hit anything. Cant spawn mina")
      (return))))