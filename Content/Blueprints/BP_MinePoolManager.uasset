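; BP_MinePoolManager is an object pool actor that pre-spawns and recycles BP_Mina mine actors.
; On BeginPlay it fills PooledEntries with deactivated mines, each paired with an availability flag and subscribed to OnMineExpired.
; GetMineFromPool claims the first free mine, or spawns another if CanExpand is set.
; ReturnMineToPool moves a mine back to the manager's location and marks it available.
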(event EventBeginPlay
  (Pooling|InitializePool))

(fn ConstructionScript)

(fn InitializePool
  (for _index (range 0 (- (Variables|Pooling|GetInitialPoolSize) 1))
    (Pooling|AddNewMinetoPool true)))

(fn GetMinefromPool
  (for (_array_element _array_index) (Variables|Pooling|GetPooledEntries)
    (if (.IsAvailable (Utilities|Struct|BreakST_MinePoolEntry _array_element))
      (Pooling|SetMineEntryat _array_index false (.Mine (Utilities|Struct|BreakST_MinePoolEntry _array_element)))
      (return (.Mine (Utilities|Struct|BreakST_MinePoolEntry _array_element)))))
  (if (Variables|Pooling|GetCanExpand)
    (bind _addedmine (Pooling|AddNewMinetoPool false))
    (return _addedmine)
    (else
      (return 0))))

(fn SpawnMine
  (bind _returnvalue (Game|SpawnActorfromClass "/Game/Blueprints/BP_Mina.BP_Mina_C" (Transformation|GetActorTransform) "AlwaysSpawn" "MultiplyWithRoot" 0 0))
  (return _returnvalue))

(fn AddNewMinetoPool
  (params (InitialAvailability :type Boolean))
  (bind _returnvalue (Pooling|SpawnMine))
  (Default|DeactivateMine _returnvalue)
  (Pooling|AddMinetoPool _returnvalue InitialAvailability)
  (return _returnvalue))

(fn AddMinetoPool
  (params (Mine :type BP%20Mina%20Object%20Reference) (IsAvailable :type Boolean))
  (Utilities|Array|Add (Variables|Pooling|GetPooledEntries) (Utilities|Struct|MakeST_MinePoolEntry IsAvailable Mine))
  ;[0.15 0.15 0.15 0.5] Subscribe to Mine expired event
  (EventDispatchers|BindEventtoOnMineExpired Mine (EventDispatchers|CreateEvent :!event ReturnMinetoPool)))

(fn ReturnMinetoPool
  (params (Mine :type BP%20Mina%20Object%20Reference))
  (for (_array_element _array_index) (Variables|Pooling|GetPooledEntries)
    (if (== Mine (.Mine (Utilities|Struct|BreakST_MinePoolEntry _array_element)))
      (Transformation|SetActorLocation (.Mine (Utilities|Struct|BreakST_MinePoolEntry _array_element)) (Transformation|GetActorLocation) false false)
      (Pooling|SetMineEntryat _array_index true (.Mine (Utilities|Struct|BreakST_MinePoolEntry _array_element)))
      (return))))

(fn SetMineEntryat
  (params (Index :type Integer) (IsAvailable :type Boolean) (Mine :type BP%20Mina%20Object%20Reference))
  (Utilities|Array|SetArrayElem (Variables|Pooling|GetPooledEntries) Index (Utilities|Struct|MakeST_MinePoolEntry IsAvailable Mine)))