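; BP_Minigun is an automatic hitscan weapon that deals fixed damage to what it hits.
; HandleFiringWeapon fires immediately and starts a looping FireRate timer to repeat shots, while DisableFiring, also called on EndPlay, clears it.
; FireWeapon line-traces on the Visibility channel from the Muzzle's forward vector, applying damage on hit.
; Debug trace drawing and hit printouts remain, with a note linking the drawing to a disappearing mirror camera.
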(event Custom|OnWeaponTimerFinished
  (Weapon|FireWeapon))

(event EventEndPlay
  (params (EndPlayReason :type EEndPlayReason%20Enum :default "Destroyed"))
  (Weapon|DisableFiring))

(fn ConstructionScript)

(fn FireWeapon
  (bind _muzzle (Variables|Default|GetMuzzle))
  (bind _returnvalue (Transformation|GetWorldLocation _muzzle))
  (if (Variables|Weapon|GetIsFiring)
    ;[0.15 0.15 0.15 0.5] TO REMOVE DEBUG DRAW TO FIX DISAPPEARING MIRROR CAMERA
    (bind (_outhit _returnvalue_2) (Collision|LineTraceByChannel _returnvalue (+ _returnvalue (* (Math|Vector|GetForwardVector _muzzle) (Variables|Weapon|GetLineTraceDistance))) "TraceTypeQuery1" false 0 "ForDuration"))
    (if _returnvalue_2
      (Development|PrintString (Utilities|GetDisplayName (.hitactor _outhit)))
      (Game|Damage|ApplyDamage (.hitactor _outhit) 1e+01 0 self)
      (else
        (Development|PrintString "Hit nothing")))))

(fn HandleFiringWeapon
  (Variables|Weapon|SetIsFiring true)
  (Weapon|FireWeapon)
  (bind _returnvalue (Utilities|Time|SetTimerbyEvent (EventDispatchers|CreateEvent :!event Custom|OnWeaponTimerFinished) (Variables|Weapon|GetFireRate) true))
  (Variables|Weapon|SetFireTimerHandle _returnvalue))

(fn DisableFiring
  (Variables|Weapon|SetIsFiring false)
  (Utilities|Time|ClearandInvalidateTimerbyHandle (Variables|Weapon|GetFireTimerHandle)))