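; Death Race game mode in which victory requires both completed laps and a target number of enemy kills.
; RegisterEnemyKilled ignores kills after the match ends, otherwise increments the count, broadcasts OnEnemyKilled with current and target totals, then re-evaluates victory.
; EvaluateVictoryConditions calls TriggerVictory only when LapsCompleted is set and the kill target is reached.
; BeginPlay and construction only call the parent.
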(event EventBeginPlay
  (|CallParentFunction))

(fn ConstructionScript
  (|CallParentFunction))

(fn RegisterEnemyKilled
  (if (Variables|Default|GetMatchEnded)
    (return)
    (else
      (bind _result (Math|Integer|IncrementInt (Variables|Default|GetEnemiesKilled))
        (:%20%20
          (Default|CallOnEnemyKilled _result (Variables|Default|GetEnemiesToKill))
          (CallFunction|EvaluateVictoryConditions))))))

(fn EvaluateVictoryConditions
  (if (Variables|Default|GetLapsCompleted)
    (if (>= (Variables|Default|GetEnemiesKilled) (Variables|Default|GetEnemiesToKill))
      (CallFunction|TriggerVictory)
      (else
        (return)))
    (else
      (return))))